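; BP_MovingTarget is a target that slides back and forth along world X, sized at BeginPlay from its Settings.
; Each Tick offsets it by Speed, unscaled by delta time, and flips direction when the Sphere's center leaves the Bounds box.
; A positive Jitter adds random reversals through a Delay in Tick, with higher Jitter mapping to longer average intervals.
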(event `self.ReceiveBeginPlay`
  (`parent.ReceiveBeginPlay`)
  (`self.SetActorScale3D` (`KismetMathLibrary.Conv_DoubleToVector` (`.Size_2_CB0E044F4C211779E916EDBF80A7DF96` (break `/Game/Blueprints/TargetSettings` (`self.Settings`))))))

(event `self.ReceiveTick`
  (params (DeltaSeconds :type "Float (single-precision)"))
  (bind _bounds (`self.Bounds`))
  (bind (_size _speed _jitter) (break `/Game/Blueprints/TargetSettings` (`self.Settings`)))
  (bind _returnvalue (`KismetMathLibrary.MapRangeClamped` _jitter 1.0 0.0 3.0 0.25))
  (bind _returnvalue_2 (/ _returnvalue 2.0))
  (`|ExecutionSequence`
    (:`then_0`
      (`self.K2_AddActorWorldOffset` (`KismetMathLibrary.MakeVector` (* _speed (select `bool` (`self.MovingLeft`) :`false` -1.0 :`true` 1.0))))
      (if (not (`KismetMathLibrary.IsPointInBox` (`SceneComponent.K2_GetComponentLocation` (`self.Sphere`)) (`SceneComponent.K2_GetComponentLocation` _bounds) (`BoxComponent.GetScaledBoxExtent` _bounds)))
        (set `self.MovingLeft` (not (`self.MovingLeft`)))))
    (:`then_1`
      (if (> _jitter 0.0)
        (`KismetSystemLibrary.Delay` (`KismetMathLibrary.RandomFloatInRange` (- _returnvalue _returnvalue_2) (+ _returnvalue_2 _returnvalue)))
        (set `self.MovingLeft` (not (`self.MovingLeft`)))))))

(fn `UserConstructionScript`
  (`parent.UserConstructionScript`))