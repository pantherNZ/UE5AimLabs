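; BP_UpgradeNPC is an NPC actor that keeps turning to face the player; no upgrade logic is present in these graphs.
; Each Tick it interpolates toward the player pawn's look-at yaw along the shortest path, scaled by RotateSpeed and delta time, with pitch and roll targeting zero.
; It then sets ShouldMove on its ABP_MPMECH anim instance whenever the raw yaw difference exceeds a small threshold.
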(event `self.ReceiveTick`
  (params (DeltaSeconds :type "Float (single-precision)"))
  (bind _returnvalue (`self.K2_GetActorRotation`))
  (bind (_returnvalue_roll _returnvalue_pitch _returnvalue_yaw) (`KismetMathLibrary.BreakRotator` (`KismetMathLibrary.FindLookAtRotation` (`self.K2_GetActorLocation`) (`self.K2_GetActorLocation` (`GameplayStatics.GetPlayerPawn` 0)))))
  (`self.K2_SetActorRotation` (`KismetMathLibrary.RLerp` _returnvalue (`KismetMathLibrary.MakeRotator` 0.0 0.0 _returnvalue_yaw) (* (`self.RotateSpeed`) (`GameplayStatics.GetWorldDeltaSeconds`)) true))
  (bind _asabp_mpmech (cast `/Game/MPMECH/BP/ABP_MPMECH` (`SkeletalMeshComponent.GetAnimInstance` (`self.SkeletalMeshComponent1`))))
  (set `/Game/MPMECH/BP/ABP_MPMECH.ShouldMove` (> (`KismetMathLibrary.Abs` (- _returnvalue_yaw (.yaw _returnvalue))) 2.0) _asabp_mpmech))

(fn `UserConstructionScript`)