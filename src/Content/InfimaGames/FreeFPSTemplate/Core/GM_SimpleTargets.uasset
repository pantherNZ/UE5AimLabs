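; Target-practice game mode that spawns BP_MovingTarget actors inside a box volume and tracks score, best score and a countdown.
; While active, Tick tops targets up to a minimum, adding more after randomized delays up to a maximum.
; Destroyed targets are detected by pruning invalid references, which scores points and starts the timer.
; Reset toggles the session and clears targets, while SetSettings remaps normalized inputs into target settings and player mouse sensitivity.
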(event `self.ReceiveBeginPlay`
  (`parent.ReceiveBeginPlay`)
  (`|ExecutionSequence`
    (:`then_0`
      (if (`|EnumEquality` (`self.SpawnMode`) "NewEnumerator0")
        (set `self.MinTargets` (`self.MaxTargets`))))))

(event `SpawnTargets`
  (bind _spawnvolume (`self.SpawnVolume`))
  (while (< (`KismetArrayLibrary.Array_Length` (`self.AllTargets`)) (`self.MinTargets`)) :!label _label
    (bind _returnvalue (`|SpawnActorFromClass` "/Game/Blueprints/BP_MovingTarget.BP_MovingTarget_C" (`KismetMathLibrary.MakeTransform` (`KismetMathLibrary.RandomPointInBoundingBox` (`SceneComponent.K2_GetComponentLocation` _spawnvolume) (`BoxComponent.GetScaledBoxExtent` _spawnvolume))) "AlwaysSpawn" "MultiplyWithRoot" null (`self.TargetSettings`) _spawnvolume null :!label _label_2))
    (`KismetArrayLibrary.Array_Add` (`self.AllTargets`) _returnvalue)))

(event `self.ReceiveTick`
  (params (DeltaSeconds :type "Float (single-precision)"))
  (`parent.ReceiveTick` DeltaSeconds)
  (`self.IfActive`
    (:`NewParam`
      (`|ExecutionSequence`
        (:`then_0`
          (`self.RemoveNullTargets`)
          (goto _label))
        (:`then_1`
          (`KismetSystemLibrary.Delay` (+ (`self.SpawnTimeSec`) (* (`self.SpawnTimeRandomSec`) (`KismetMathLibrary.RandomFloat`))))
          (if (< (`KismetArrayLibrary.Array_Length` (`self.AllTargets`)) (`self.MaxTargets`))
            (goto _label_2)))
        (:`then_2`
          (if (`self.IsTicking`)
            (bind _output_get (set `self.Timer` (`KismetMathLibrary.FMax` (- (`self.Timer`) (`GameplayStatics.GetWorldDeltaSeconds`)))))
            (set `self.IsTicking` (> _output_get 0.0))))))))

(event `Reset`
  (bind _alltargets (`self.AllTargets`))
  (set `self.Timer` 20.0)
  (set `self.Score` 0)
  (set `self.IsTicking` false)
  (bind _output_get (set `self.IsActive` (not (`self.IsActive`))))
  (for _array_element _alltargets
    (`self.K2_DestroyActor` _array_element)
    (`KismetArrayLibrary.Array_Clear` _alltargets)
    (if _output_get
      (`self.SpawnTargets`))))

(fn `RemoveNullTargets`
  (bind _alltargets (`self.AllTargets`))
  (bind (_arrayindex _arrayelement) (`/Engine/EditorBlueprintResources/StandardMacros.ReverseForEachLoop` _alltargets)
    (:`LoopBody`
      (`/Engine/EditorBlueprintResources/StandardMacros.IsValid` _arrayelement
        (:`Is Not Valid`
          (`KismetArrayLibrary.Array_Remove` _alltargets _arrayindex)
          (bind _result (`/Engine/EditorBlueprintResources/StandardMacros.IncrementInt` (`self.Score`))
            (:`  `
              (set `self.BestScore` (`KismetMathLibrary.Max` _result (`self.BestScore`)))
              (set `self.IsTicking` true))))))))

(fn `SetSettings`
  (params (RawSettings :type "/Game/Blueprints/TargetSettings Structure"))
  (bind (_size _speed _jitter _sensitivity) (break `/Game/Blueprints/TargetSettings` RawSettings))
  (bind _returnvalue (`KismetMathLibrary.MapRangeClamped` _sensitivity 0.0 1.0 0.1 5.0))
  (set `self.TargetSettings` (make `/Game/Blueprints/TargetSettings` (`KismetMathLibrary.MapRangeClamped` _size 0.0 1.0 0.5 5.0) (`KismetMathLibrary.MapRangeClamped` _speed 0.0 1.0 0.0 20.0) (`KismetMathLibrary.MapRangeClamped` _jitter 0.0 1.0 0.0 1.0) _returnvalue))
  (bind _asbp_character (cast `/Game/InfimaGames/FreeFPSTemplate/Core/BP_Character` (`GameplayStatics.GetPlayerCharacter` 0)))
  (set `/Game/InfimaGames/FreeFPSTemplate/Core/BP_Character.MouseSensivity` _returnvalue _asbp_character))

(fn `UserConstructionScript`
  (`parent.UserConstructionScript`))